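; BP_PlayerShip is the player ship Blueprint, which here handles only cosmetic idle animation on Tick.
; The Reactive effect component pulses along its Y scale, driven by a looping sawtooth lerp that grows and snaps back about five times a second.
; The Hull rocks in pitch at a constant rate, reversing direction whenever it reaches either angle limit.
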(event `self.ReceiveTick`
  (params (DeltaSeconds :type "Float (single-precision)"))
  (bind _hull (`self.Hull`))
  (bind _returnvalue (+ (* DeltaSeconds 5.0) (`self.ReactiveEffectLerp`)))
  (bind _pitch (.pitch (`SceneComponent.RelativeRotation` _hull)))
  ;[1 1 1] Reactive Effect
  (if (> _returnvalue 1.0)
    (set `self.ReactiveEffectLerp` 0.0)
    (else
      (bind _output_get (set `self.ReactiveEffectLerp` _returnvalue))))
  (`SceneComponent.SetRelativeScale3D` (`self.Reactive`) (`KismetMathLibrary.MakeVector` 1.0 (`KismetMathLibrary.Lerp` 0.9 1.1 _output_get) 1.0))
  ;[1 1 1] Hull Rotation
  (if (<= _pitch -10.0)
    (set `self.HullRotationDirection` 10.0)
    (elif (>= _pitch 10.0)
      (set `self.HullRotationDirection` -10.0)))
  (`SceneComponent.K2_AddRelativeRotation` _hull (`KismetMathLibrary.MakeRotator` 0.0 (* (`self.HullRotationDirection`) (`GameplayStatics.GetWorldDeltaSeconds`))) false false))

(fn `UserConstructionScript`)